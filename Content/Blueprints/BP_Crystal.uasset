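; BP_Crystal is an actor with two crystal components that bob up and down, plus a sound player.
; Every Tick drives each crystal's relative Z with a sine of game time, using slightly different speeds and amplitudes and opposite sign so they float out of step.
; The construction script assigns the CrystalSound variable to the Soundplayer component, so the sound is configurable on the actor.
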(event `self.ReceiveTick`
  (params (DeltaSeconds :type "Float (single-precision)"))
  (bind _returnvalue (`self.GetGameTimeSinceCreation`))
  (`SceneComponent.K2_SetRelativeLocation` (`self.crystal`) (`KismetMathLibrary.MakeVector` 0.0 0.0 (* (`KismetMathLibrary.Sin` (* _returnvalue 0.5)) 40.0)) false false)
  (`SceneComponent.K2_SetRelativeLocation` (`self.crystal1`) (`KismetMathLibrary.MakeVector` 0.0 0.0 (* (* (`KismetMathLibrary.Sin` (* _returnvalue 0.6)) 30.0) -1.0)) false false))

(fn `UserConstructionScript`
  (`AudioComponent.SetSound` (`self.soundplayer`) (`self.CrystalSound`)))
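; BP_MAIN_Crystal is a crystal actor that bobs up and down and carries a sound player.
; On Tick it sets the relative location of its Kristalisierendbad component along Z, using a slow sine wave driven by game time since creation.
; The construction script assigns the CrystalSound variable to the Soundplayer component, so the sound can differ per instance.
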(event `self.ReceiveTick`
  (params (DeltaSeconds :type "Float (single-precision)"))
  (`SceneComponent.K2_SetRelativeLocation` (`self.kristalisierend-bad`) (`KismetMathLibrary.MakeVector` 0.0 0.0 (* (`KismetMathLibrary.Sin` (* (`self.GetGameTimeSinceCreation`) 0.5)) 40.0)) false false))

(fn `UserConstructionScript`
  (`AudioComponent.SetSound` (`self.soundplayer`) (`self.CrystalSound`)))
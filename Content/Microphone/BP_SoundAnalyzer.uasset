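; BP_SoundAnalyzer is an actor that creates a render target at BeginPlay and displays it on its Canvas component.
; It clears the target to off-white and draws a single pink diagonal test line through the Canvas draw API.
; A dynamic instance of CanvasMaterial receives the target as a texture parameter and is applied to the component.
; Despite the name, it contains no audio capture or analysis logic.
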(event `self.ReceiveBeginPlay`
  (`|ExecutionSequence`
    (:`then_0`
      (bind _returnvalue (`KismetRenderingLibrary.CreateRenderTarget2D` 1024 1024))
      (bind _output_get (set `self.RenderTarget` _returnvalue))
      (`KismetRenderingLibrary.ClearRenderTarget2D` _output_get (struct :`R` 1.0 :`G` 0.976277 :`B` 0.933301 :`A` 1.0))
      (bind (_canvas _size _context) (`KismetRenderingLibrary.BeginDrawCanvasToRenderTarget` _output_get))
      (`Canvas.K2_DrawLine` _canvas (0.0 0.0) (1000.0 1000.0) 5.0 (struct :`R` 1.0 :`G` 0.042006 :`B` 0.732362 :`A` 1.0))
      (`KismetRenderingLibrary.EndDrawCanvasToRenderTarget` _context))
    (:`then_1`
      (bind _returnvalue_2 (`KismetMaterialLibrary.CreateDynamicMaterialInstance` "/Game/Microphone/CanvasMaterial.CanvasMaterial"))
      (`MaterialInstanceDynamic.SetTextureParameterValue` _returnvalue_2 "Rendertarget" (`self.RenderTarget`))
      (`PrimitiveComponent.SetMaterial` (`self.Canvas`) 0 _returnvalue_2))))

(fn `UserConstructionScript`)